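; Green keypad puzzle with nine physically pushed keys that sets Solved when 3, 9, 5 is entered in order.
; A key's begin overlap stores the touching component, its start location and the key's number.
; Tick moves that key by the component's clamped local Z travel, or interpolates it back when none is stored.
; Full depth registers one press through a DoOnce, advancing or clearing the First and Second progress flags.
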(event `self.key_1.OnComponentBeginOverlap`
  (params (OverlappedComponent :type "PrimitiveComponent Object Reference") (OtherActor :type "Actor Object Reference") (OtherComp :type "PrimitiveComponent Object Reference") (OtherBodyIndex :type Integer) (bFromSweep :type Boolean) (SweepResult :type "HitResult Structure (by ref)"))
  (`/Engine/EditorBlueprintResources/StandardMacros.IsValid` (`self.OverlappedComponent`)
    (:`Is Not Valid`
      (bind _output_get (set `self.OverlappedComponent` OtherComp))
      (set `self.InitialOverlapLocation` (`SceneComponent.K2_GetComponentLocation` _output_get))
      (set `self.ThisComponent` OverlappedComponent)
      (set `self.InputNum` 1))))

(event `self.key_2.OnComponentBeginOverlap`
  (params (OverlappedComponent :type "PrimitiveComponent Object Reference") (OtherActor :type "Actor Object Reference") (OtherComp :type "PrimitiveComponent Object Reference") (OtherBodyIndex :type Integer) (bFromSweep :type Boolean) (SweepResult :type "HitResult Structure (by ref)"))
  (`/Engine/EditorBlueprintResources/StandardMacros.IsValid` (`self.OverlappedComponent`)
    (:`Is Not Valid`
      (bind _output_get (set `self.OverlappedComponent` OtherComp))
      (set `self.InitialOverlapLocation` (`SceneComponent.K2_GetComponentLocation` _output_get))
      (set `self.ThisComponent` OverlappedComponent)
      (set `self.InputNum` 2))))

(event `self.key_3.OnComponentBeginOverlap`
  (params (OverlappedComponent :type "PrimitiveComponent Object Reference") (OtherActor :type "Actor Object Reference") (OtherComp :type "PrimitiveComponent Object Reference") (OtherBodyIndex :type Integer) (bFromSweep :type Boolean) (SweepResult :type "HitResult Structure (by ref)"))
  (`/Engine/EditorBlueprintResources/StandardMacros.IsValid` (`self.OverlappedComponent`)
    (:`Is Not Valid`
      (bind _output_get (set `self.OverlappedComponent` OtherComp))
      (set `self.InitialOverlapLocation` (`SceneComponent.K2_GetComponentLocation` _output_get))
      (set `self.ThisComponent` OverlappedComponent)
      (set `self.InputNum` 3))))

(event `self.ReceiveTick`
  (params (DeltaSeconds :type "Float (single-precision)"))
  (bind _thiscomponent (`self.ThisComponent`))
  (bind (_returnvalue_x _returnvalue_y _returnvalue_z) (`KismetMathLibrary.BreakVector` (- (`KismetMathLibrary.InverseTransformLocation` (`SceneComponent.K2_GetComponentToWorld` _thiscomponent) (`self.InitialOverlapLocation`)) (`KismetMathLibrary.InverseTransformLocation` (`SceneComponent.K2_GetComponentToWorld` _thiscomponent) (`SceneComponent.K2_GetComponentLocation` (`self.OverlappedComponent`))))))
  (`|ExecutionSequence`
    (:`then_0`
      (`/Engine/EditorBlueprintResources/StandardMacros.IsValid` (`self.OverlappedComponent`)
        (:`Is Valid`
          (bind _output_get (set `self.ButtonPressAmount` (`KismetMathLibrary.FClamp` _returnvalue_z 0.0 (`self.MaxButtonPressAmount`))))
          (`SceneComponent.K2_SetRelativeLocation` (`self.ThisComponent`) (`KismetMathLibrary.MakeVector` 0.0 0.0 (* _output_get -1.0)) false false))
        (:`Is Not Valid`
          (`SceneComponent.K2_SetRelativeLocation` (`self.ThisComponent`) (`KismetMathLibrary.VInterpTo` (`SceneComponent.RelativeLocation` (`self.ThisComponent`)) (0.0 0.0 0.0) DeltaSeconds 10.0) false false))))
    (:`then_1`
      (if (>= (`self.ButtonPressAmount`) (`self.MaxButtonPressAmount`))
        (`/Engine/EditorBlueprintResources/StandardMacros.DoOnce` false :!label _label
          (:`Completed`
            (if (`self.First`)
              (if (`self.Second`)
                (if (== (`self.InputNum`) 5)
                  (set `self.Solved` true)
                  (else
                    (set `self.First` false)
                    (set `self.Second` false)))
                (elif (== (`self.InputNum`) 9)
                  (set `self.Second` true)
                  (else
                    (set `self.First` false))))
              (elif (== (`self.InputNum`) 3)
                (set `self.First` true)))))
        (else
          (goto _label :!via `Reset`))))))

(event `self.key_4.OnComponentBeginOverlap`
  (params (OverlappedComponent :type "PrimitiveComponent Object Reference") (OtherActor :type "Actor Object Reference") (OtherComp :type "PrimitiveComponent Object Reference") (OtherBodyIndex :type Integer) (bFromSweep :type Boolean) (SweepResult :type "HitResult Structure (by ref)"))
  (`/Engine/EditorBlueprintResources/StandardMacros.IsValid` (`self.OverlappedComponent`)
    (:`Is Not Valid`
      (bind _output_get (set `self.OverlappedComponent` OtherComp))
      (set `self.InitialOverlapLocation` (`SceneComponent.K2_GetComponentLocation` _output_get))
      (set `self.ThisComponent` OverlappedComponent)
      (set `self.InputNum` 4))))

(event `self.key_5.OnComponentBeginOverlap`
  (params (OverlappedComponent :type "PrimitiveComponent Object Reference") (OtherActor :type "Actor Object Reference") (OtherComp :type "PrimitiveComponent Object Reference") (OtherBodyIndex :type Integer) (bFromSweep :type Boolean) (SweepResult :type "HitResult Structure (by ref)"))
  (`/Engine/EditorBlueprintResources/StandardMacros.IsValid` (`self.OverlappedComponent`)
    (:`Is Not Valid`
      (bind _output_get (set `self.OverlappedComponent` OtherComp))
      (set `self.InitialOverlapLocation` (`SceneComponent.K2_GetComponentLocation` _output_get))
      (set `self.ThisComponent` OverlappedComponent)
      (set `self.InputNum` 5))))

(event `self.key_6.OnComponentBeginOverlap`
  (params (OverlappedComponent :type "PrimitiveComponent Object Reference") (OtherActor :type "Actor Object Reference") (OtherComp :type "PrimitiveComponent Object Reference") (OtherBodyIndex :type Integer) (bFromSweep :type Boolean) (SweepResult :type "HitResult Structure (by ref)"))
  (`/Engine/EditorBlueprintResources/StandardMacros.IsValid` (`self.OverlappedComponent`)
    (:`Is Not Valid`
      (bind _output_get (set `self.OverlappedComponent` OtherComp))
      (set `self.InitialOverlapLocation` (`SceneComponent.K2_GetComponentLocation` _output_get))
      (set `self.ThisComponent` OverlappedComponent)
      (set `self.InputNum` 6))))

(event `self.key_7.OnComponentBeginOverlap`
  (params (OverlappedComponent :type "PrimitiveComponent Object Reference") (OtherActor :type "Actor Object Reference") (OtherComp :type "PrimitiveComponent Object Reference") (OtherBodyIndex :type Integer) (bFromSweep :type Boolean) (SweepResult :type "HitResult Structure (by ref)"))
  (`/Engine/EditorBlueprintResources/StandardMacros.IsValid` (`self.OverlappedComponent`)
    (:`Is Not Valid`
      (bind _output_get (set `self.OverlappedComponent` OtherComp))
      (set `self.InitialOverlapLocation` (`SceneComponent.K2_GetComponentLocation` _output_get))
      (set `self.ThisComponent` OverlappedComponent)
      (set `self.InputNum` 7))))

(event `self.key_8.OnComponentBeginOverlap`
  (params (OverlappedComponent :type "PrimitiveComponent Object Reference") (OtherActor :type "Actor Object Reference") (OtherComp :type "PrimitiveComponent Object Reference") (OtherBodyIndex :type Integer) (bFromSweep :type Boolean) (SweepResult :type "HitResult Structure (by ref)"))
  (`/Engine/EditorBlueprintResources/StandardMacros.IsValid` (`self.OverlappedComponent`)
    (:`Is Not Valid`
      (bind _output_get (set `self.OverlappedComponent` OtherComp))
      (set `self.InitialOverlapLocation` (`SceneComponent.K2_GetComponentLocation` _output_get))
      (set `self.ThisComponent` OverlappedComponent)
      (set `self.InputNum` 8))))

(event `self.key_9.OnComponentBeginOverlap`
  (params (OverlappedComponent :type "PrimitiveComponent Object Reference") (OtherActor :type "Actor Object Reference") (OtherComp :type "PrimitiveComponent Object Reference") (OtherBodyIndex :type Integer) (bFromSweep :type Boolean) (SweepResult :type "HitResult Structure (by ref)"))
  (`/Engine/EditorBlueprintResources/StandardMacros.IsValid` (`self.OverlappedComponent`)
    (:`Is Not Valid`
      (bind _output_get (set `self.OverlappedComponent` OtherComp))
      (set `self.InitialOverlapLocation` (`SceneComponent.K2_GetComponentLocation` _output_get))
      (set `self.ThisComponent` OverlappedComponent)
      (set `self.InputNum` 9))))

(event `self.key_1.OnComponentEndOverlap`
  (params (OverlappedComponent :type "PrimitiveComponent Object Reference") (OtherActor :type "Actor Object Reference") (OtherComp :type "PrimitiveComponent Object Reference") (OtherBodyIndex :type Integer))
  (if (== OtherComp (`self.DefaultSceneRoot`))
    (set `self.OverlappedComponent` null)))

(event `self.key_2.OnComponentEndOverlap`
  (params (OverlappedComponent :type "PrimitiveComponent Object Reference") (OtherActor :type "Actor Object Reference") (OtherComp :type "PrimitiveComponent Object Reference") (OtherBodyIndex :type Integer))
  (if (== OtherComp (`self.DefaultSceneRoot`))
    (set `self.OverlappedComponent` null)))

(event `self.key_3.OnComponentEndOverlap`
  (params (OverlappedComponent :type "PrimitiveComponent Object Reference") (OtherActor :type "Actor Object Reference") (OtherComp :type "PrimitiveComponent Object Reference") (OtherBodyIndex :type Integer))
  (if (== OtherComp (`self.DefaultSceneRoot`))
    (set `self.OverlappedComponent` null)))

(event `self.key_4.OnComponentEndOverlap`
  (params (OverlappedComponent :type "PrimitiveComponent Object Reference") (OtherActor :type "Actor Object Reference") (OtherComp :type "PrimitiveComponent Object Reference") (OtherBodyIndex :type Integer))
  (if (== OtherComp (`self.DefaultSceneRoot`))
    (set `self.OverlappedComponent` null)))

(event `self.key_5.OnComponentEndOverlap`
  (params (OverlappedComponent :type "PrimitiveComponent Object Reference") (OtherActor :type "Actor Object Reference") (OtherComp :type "PrimitiveComponent Object Reference") (OtherBodyIndex :type Integer))
  (if (== OtherComp (`self.DefaultSceneRoot`))
    (set `self.OverlappedComponent` null)))

(event `self.key_6.OnComponentEndOverlap`
  (params (OverlappedComponent :type "PrimitiveComponent Object Reference") (OtherActor :type "Actor Object Reference") (OtherComp :type "PrimitiveComponent Object Reference") (OtherBodyIndex :type Integer))
  (if (== OtherComp (`self.DefaultSceneRoot`))
    (set `self.OverlappedComponent` null)))

(event `self.key_7.OnComponentEndOverlap`
  (params (OverlappedComponent :type "PrimitiveComponent Object Reference") (OtherActor :type "Actor Object Reference") (OtherComp :type "PrimitiveComponent Object Reference") (OtherBodyIndex :type Integer))
  (if (== OtherComp (`self.DefaultSceneRoot`))
    (set `self.OverlappedComponent` null)))

(event `self.key_8.OnComponentEndOverlap`
  (params (OverlappedComponent :type "PrimitiveComponent Object Reference") (OtherActor :type "Actor Object Reference") (OtherComp :type "PrimitiveComponent Object Reference") (OtherBodyIndex :type Integer))
  (if (== OtherComp (`self.DefaultSceneRoot`))
    (set `self.OverlappedComponent` null)))

(event `self.key_9.OnComponentEndOverlap`
  (params (OverlappedComponent :type "PrimitiveComponent Object Reference") (OtherActor :type "Actor Object Reference") (OtherComp :type "PrimitiveComponent Object Reference") (OtherBodyIndex :type Integer))
  (if (== OtherComp (`self.DefaultSceneRoot`))
    (set `self.OverlappedComponent` null)))

(fn `UserConstructionScript`)