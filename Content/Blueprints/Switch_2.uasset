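; Physical push-button switch actor whose Swtich component sinks as an overlapping component pushes it down.
; Begin overlap stores the component and its starting location; Tick converts its movement into Scene-local Z depth, clamped to MaxButtonPressAmount.
; Without a tracked component the button interpolates back, though end overlap clears tracking only when the other component equals DefaultSceneRoot.
; A DoOnce latches at full press and resets below it, but triggers nothing yet.
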(event `self.ReceiveTick`
  (params (DeltaSeconds :type "Float (single-precision)"))
  (bind _scene (`self.Scene`))
  (bind (_returnvalue_x _returnvalue_y _returnvalue_z) (`KismetMathLibrary.BreakVector` (- (`KismetMathLibrary.InverseTransformLocation` (`SceneComponent.K2_GetComponentToWorld` _scene) (`self.InitialOverlapLocation`)) (`KismetMathLibrary.InverseTransformLocation` (`SceneComponent.K2_GetComponentToWorld` _scene) (`SceneComponent.K2_GetComponentLocation` (`self.OverlappedComponent`))))))
  (`|ExecutionSequence`
    (:`then_0`
      (`/Engine/EditorBlueprintResources/StandardMacros.IsValid` (`self.OverlappedComponent`)
        (:`Is Valid`
          (bind _output_get (set `self.ButtonPressAmount` (`KismetMathLibrary.FClamp` _returnvalue_z 0.0 (`self.MaxButtonPressAmount`))))
          (`SceneComponent.K2_SetRelativeLocation` (`self.Swtich`) (`KismetMathLibrary.MakeVector` 0.0 0.0 (* _output_get -1.0)) false false))
        (:`Is Not Valid`
          (`SceneComponent.K2_SetRelativeLocation` (`self.Swtich`) (`KismetMathLibrary.VInterpTo` (`SceneComponent.RelativeLocation` (`self.Swtich`)) (0.0 0.0 0.0) DeltaSeconds 10.0) false false))))
    (:`then_1`
      (if (>= (`self.ButtonPressAmount`) (`self.MaxButtonPressAmount`))
        (`/Engine/EditorBlueprintResources/StandardMacros.DoOnce` false :!label _label)
        (else
          (goto _label :!via `Reset`))))))

(event `self.Swtich.OnComponentBeginOverlap`
  (params (OverlappedComponent :type "PrimitiveComponent Object Reference") (OtherActor :type "Actor Object Reference") (OtherComp :type "PrimitiveComponent Object Reference") (OtherBodyIndex :type Integer) (bFromSweep :type Boolean) (SweepResult :type "HitResult Structure (by ref)"))
  (`/Engine/EditorBlueprintResources/StandardMacros.IsValid` (`self.OverlappedComponent`)
    (:`Is Not Valid`
      (bind _output_get (set `self.OverlappedComponent` OtherComp))
      (set `self.InitialOverlapLocation` (`SceneComponent.K2_GetComponentLocation` _output_get)))))

(event `self.Swtich.OnComponentEndOverlap`
  (params (OverlappedComponent :type "PrimitiveComponent Object Reference") (OtherActor :type "Actor Object Reference") (OtherComp :type "PrimitiveComponent Object Reference") (OtherBodyIndex :type Integer))
  (if (== OtherComp (`self.DefaultSceneRoot`))
    (set `self.OverlappedComponent` null)))

(fn `UserConstructionScript`)