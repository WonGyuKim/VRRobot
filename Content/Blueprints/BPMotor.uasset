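; BPMotor is a motor actor that acts as a rotation source for the objects linked to it.
; While IsRotate is on, each Tick spins its static mesh around the mesh's up vector by RotationAngle, without scaling by delta time.
; It then passes itself, the angle and that axis to every LinkList entry through TransferRotation.
; ToggleEnable flips IsRotate to start or stop the motor.
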(event `self.ReceiveTick`
  (params (DeltaSeconds :type "Float (single-precision)"))
  (`parent.ReceiveTick` DeltaSeconds)
  (`self.MotorRotation`))

(fn `MotorRotation`
  (bind _staticmesh (`self.StaticMesh`))
  (if (`self.IsRotate`)
    (`SceneComponent.K2_AddWorldRotation` _staticmesh (`KismetMathLibrary.RotatorFromAxisAndAngle` (`SceneComponent.GetUpVector` _staticmesh) (`self.RotationAngle`)) false false)
    (for _array_element (`self.LinkList`)
      (`/Game/Blueprints/Link/BPLink.TransferRotation` _array_element self (`self.RotationAngle`) (`SceneComponent.GetUpVector` (`self.StaticMesh`))))
    (return)))

(fn `ToggleEnable`
  (set `self.IsRotate` (not (`self.IsRotate`)))
  (return))

(fn `UserConstructionScript`
  (`parent.UserConstructionScript`))