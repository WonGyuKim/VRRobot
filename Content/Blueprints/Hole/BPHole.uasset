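; BPHole is a hole attached to a parent BPComponents actor that aligns it with another component inserted into the hole.
; Overlap records one entering component and registers the hole with the hand holding either part, preferring the parent's.
; WhenHandRelease calls InterpolatingLocation, then unregisters the hole.
; Despite its name, that function instantly moves the held part's mesh onto the other's up axis, using vector projection to preserve axial offset.
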(event `self.ReceiveBeginPlay`
  (bind _asbpcomponents (cast `/Game/Blueprints/BPComponents` (`self.GetParentActor`)))
  (set `self.ParentActor` _asbpcomponents))

(event `self.ReceiveActorBeginOverlap`
  (params (OtherActor :type "Actor Object Reference"))
  (bind _asbpcomponents (cast `/Game/Blueprints/BPComponents` OtherActor))
  (`self.StartOverlap` _asbpcomponents))

(event `self.ReceiveActorEndOverlap`
  (params (OtherActor :type "Actor Object Reference"))
  (bind _asbpcomponents (cast `/Game/Blueprints/BPComponents` OtherActor))
  (`self.EndOverlap` _asbpcomponents))

(fn `EndOverlap`
  (params (InputObject :type "/Game/Blueprints/BPComponents Object Reference"))
  (if (== InputObject (`self.EnteredActor`))
    (`/Game/Blueprints/BPHand.RemoveHole` (`self.BPHand`) self)
    (set `self.BPHand` null)
    (set `self.IsEntered` false)
    (set `self.HandSide` "")
    (return)))

(fn `InterpolatingLocation`
  (bind _staticmesh (`/Game/Blueprints/BPComponents.StaticMesh` (`self.EnteredActor`)))
  (bind _capsule (`self.Capsule`))
  (bind _staticmesh_2 (`/Game/Blueprints/BPComponents.StaticMesh` (`self.EnteredActor`)))
  (bind _staticmesh_3 (`/Game/Blueprints/BPComponents.StaticMesh` (`self.ParentActor`)))
  (bind _returnvalue (- (`SceneComponent.K2_GetComponentLocation` _staticmesh_2) (`SceneComponent.K2_GetComponentLocation` (`self.Capsule`))))
  (bind _returnvalue_2 (- (`SceneComponent.K2_GetComponentLocation` _capsule) (`SceneComponent.K2_GetComponentLocation` (`/Game/Blueprints/BPComponents.StaticMesh` (`self.EnteredActor`)))))
  (bind _hand (`/Game/Blueprints/BPComponents.GetHand` (`self.ParentActor`)))
  (if (`KismetSystemLibrary.IsValid` _hand)
    ;[1 1 1] When We Control the object that has hole
    (`SceneComponent.K2_SetWorldLocation` _staticmesh_3 (+ (- _returnvalue (`KismetMathLibrary.ProjectVectorOnToVector` _returnvalue (`SceneComponent.GetUpVector` _staticmesh_2))) (`SceneComponent.K2_GetComponentLocation` _staticmesh_3)) false false)
    (else
      ;[1 1 1] When We Control the object that has no hole
      (`SceneComponent.K2_SetWorldLocation` _staticmesh (+ (`SceneComponent.K2_GetComponentLocation` _staticmesh) (- _returnvalue_2 (`KismetMathLibrary.ProjectVectorOnToVector` _returnvalue_2 (`SceneComponent.GetUpVector` _capsule)))) false false)))
  (return))

(fn `StartOverlap`
  (params (InputObject :type "/Game/Blueprints/BPComponents Object Reference"))
  (if (not (`self.IsEntered`))
    (set `self.IsEntered` true)
    (set `self.EnteredActor` InputObject)
    (bind _hand (`/Game/Blueprints/BPComponents.GetHand` (`self.ParentActor`)))
    (if (`KismetSystemLibrary.IsValid` _hand)
      (bind (_hand_2 _side) (`/Game/Blueprints/BPComponents.GetHand` (`self.ParentActor`)))
      (set `self.BPHand` _hand_2)
      (set `self.HandSide` _side)
      (else
        (bind (_hand_3 _side_2) (`/Game/Blueprints/BPComponents.GetHand` (`self.EnteredActor`)))
        (set `self.BPHand` _hand_3)
        (set `self.HandSide` _side_2)))
    (`/Game/Blueprints/BPHand.AddHole` (`self.BPHand`) self)
    (return)))

(fn `UserConstructionScript`)

(fn `WhenHandRelease`
  (params (HandSide :type String))
  (if (`KismetStringLibrary.EqualEqual_StrStr` HandSide (`self.HandSide`))
    (if (`self.IsEntered`)
      (`self.InterpolatingLocation`)
      (`/Game/Blueprints/BPHand.RemoveHole` (`self.BPHand`) self)
      (return))))