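; BPComponents is a base-style actor Blueprint that tracks a tag, a holding hand and links to other objects.
; BeginPlay calls SetTag, which is an empty stub here, and GetTag returns the stored Tag.
; SetHand and GetHand store and return a hand reference with its side.
; Link and LinkExit maintain LinkList, setting IsConnected on linking and clearing it when the list empties.
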(event `self.ReceiveBeginPlay`
  (`self.SetTag`))

(event `self.ReceiveActorEndOverlap`
  (params (OtherActor :type "Actor Object Reference")))

(fn `GetHand`
  (returns (Hand :type "/Game/Blueprints/BPHand Object Reference") (Side :type String))
  (return (`self.BPHand`) (`self.HandSide`)))

(fn `GetTag`
  (returns (Tag :type String))
  (return (`self.Tag`)))

(fn `Link`
  (params (Link :type "/Game/Blueprints/Link/BPLink Object Reference"))
  (`KismetArrayLibrary.Array_Add` (`self.LinkList`) Link)
  (if (not (`self.IsConnected`))
    (set `self.IsConnected` true)
    (return)))

(fn `LinkExit`
  (params (link :type "/Game/Blueprints/Link/BPLink Object Reference"))
  (`KismetArrayLibrary.Array_RemoveItem` (`self.LinkList`) link)
  (if (== (`KismetArrayLibrary.Array_Length` (`self.LinkList`)) 0)
    (set `self.IsConnected` false)
    (return)))

(fn `SetHand`
  (params (Hand :type "/Game/Blueprints/BPHand Object Reference") (Side :type String))
  (set `self.BPHand` Hand)
  (set `self.HandSide` Side)
  (return))

(fn `SetTag`
  (return))

(fn `UserConstructionScript`)