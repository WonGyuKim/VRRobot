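; BPLink is a link object joining two components, Left and Right, that can move one when the other rotates.
; Connect and Disconnect register and unregister the link on both ends, and Has matches a pair in either order.
; ChainingRotationMove treats the non-parent end as child and orbits its mesh location around the parent position, without propagating further.
; TransferRotation is an empty stub.
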(fn `ChainingRotationMove`
  (params (Parent :type "/Game/Blueprints/BPComponents Object Reference") (ParentPosition :type "Vector Structure") (ChainingRotateVector :type "Vector Structure") (Angle :type "Float (double-precision)") (Axis :type "Vector Structure"))
  ;[1 1 1] 이 부분 수정하세요
  (if (== Parent (`self.Left`))
    ;[1 1 1] Right is child
    (`SceneComponent.K2_SetWorldLocation` (`/Game/Blueprints/BPComponents.StaticMesh` (`self.Right`)) (+ (`KismetMathLibrary.RotateAngleAxis` (- (`SceneComponent.K2_GetComponentLocation` (`/Game/Blueprints/BPComponents.StaticMesh` (`self.Right`))) ParentPosition) Angle Axis) ParentPosition) false false)
    (else
      ;[1 1 1] Left is child
      (`SceneComponent.K2_SetWorldLocation` (`/Game/Blueprints/BPComponents.StaticMesh` (`self.Left`)) (+ ParentPosition (`KismetMathLibrary.RotateAngleAxis` (- (`SceneComponent.K2_GetComponentLocation` (`/Game/Blueprints/BPComponents.StaticMesh` (`self.Left`))) ParentPosition) Angle Axis)) false false))))

(fn `Connect`
  (params (Left :type "/Game/Blueprints/BPComponents Object Reference") (Right :type "/Game/Blueprints/BPComponents Object Reference"))
  (bind _output_get (set `self.Left` Left))
  (`/Game/Blueprints/BPComponents.Link` _output_get self)
  (bind _output_get_2 (set `self.Right` Right))
  (`/Game/Blueprints/BPComponents.Link` _output_get_2 self)
  (return))

(fn `Disconnect`
  (`/Game/Blueprints/BPComponents.LinkExit` (`self.Left`) self)
  (`/Game/Blueprints/BPComponents.LinkExit` (`self.Right`) self)
  (return))

(fn `Has`
  (params (Components1 :type "/Game/Blueprints/BPComponents Object Reference") (Components2 :type "/Game/Blueprints/BPComponents Object Reference"))
  (returns (Has :type Boolean))
  (if (or (and (== (`self.Left`) Components1) (== Components2 (`self.Right`))) (and (== Components2 (`self.Left`)) (== Components1 (`self.Right`))))
    (return true)
    (else
      (return false))))

(fn `TransferRotation`
  (params (Parent :type "/Game/Blueprints/BPComponents Object Reference") (Angle :type "Float (double-precision)") (Axis :type "Vector Structure"))
  (return))