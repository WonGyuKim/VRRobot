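; BPLink2 is a Blueprint link object that joins a Parent and a Target.
; Connect stores both references, calls Link on each with itself so both ends register the connection, then prints their names in red as long-lived debug text.
; Disconnect is an empty stub, and the event graph and construction script hold no logic.
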(fn `Connect`
  (params (parent :type "/Game/Blueprints/BPComponents Object Reference") (target :type "/Game/Blueprints/BPComponents Object Reference"))
  (bind _output_get (set `self.Parent` parent))
  (`/Game/Blueprints/BPComponents.Link` _output_get self)
  (bind _output_get_2 (set `self.Target` target))
  (`/Game/Blueprints/BPComponents.Link` _output_get_2 self)
  (`KismetSystemLibrary.PrintString` (`KismetSystemLibrary.GetObjectName` (`self.Parent`)) true true (struct :`R` 1.0 :`A` 1.0) 100.0)
  (`KismetSystemLibrary.PrintString` "and" true true (struct :`R` 1.0 :`A` 1.0) 100.0)
  (`KismetSystemLibrary.PrintString` (`KismetSystemLibrary.GetObjectName` (`self.Target`)) true true (struct :`R` 1.0 :`A` 1.0) 100.0)
  (return))

(fn `Disconnect`)

(fn `UserConstructionScript`)