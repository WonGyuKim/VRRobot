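; BPGear is a gear component, tagged "gear", that automatically links itself to other gears it touches.
; At BeginPlay it scans the gears overlapping its static mesh and creates a BPGearLink for each pair not already found in the other gear's LinkList.
; At runtime, overlapping another gear creates a link only while BPHand is valid, and ending the overlap disconnects the matching links.
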(event `self.ReceiveBeginPlay`
  (`parent.ReceiveBeginPlay`)
  (for _array_element (`PrimitiveComponent.GetOverlappingActors` (`self.StaticMesh`) "BPGear_C")
    (bind _asbpgear (cast `/Game/Blueprints/Gear/BPGear` _array_element))
    (for _array_element_2 (`/Game/Blueprints/BPComponents.LinkList` _asbpgear)
      (bind _has (`/Game/Blueprints/Link/BPLink.Has` _array_element_2 self _asbpgear))
      (if _has
        (set `self.CheckAlreadyConnectWhenStarts` true)))
    (if (`self.CheckAlreadyConnectWhenStarts`)
      (set `self.CheckAlreadyConnectWhenStarts` false)
      (else
        (`self.ConnectGearWhenStarts` _asbpgear)))))

(event `self.SetTag`
  (set `self.Tag` "gear"))

(event `self.ReceiveActorBeginOverlap`
  (params (OtherActor :type "Actor Object Reference"))
  (bind _asbpcomponents (cast `/Game/Blueprints/BPComponents` OtherActor))
  (`self.ConnectGear` _asbpcomponents))

(event `self.ReceiveActorEndOverlap`
  (params (OtherActor :type "Actor Object Reference"))
  (bind _asbpcomponents (cast `/Game/Blueprints/BPComponents` OtherActor))
  (if (`KismetStringLibrary.EqualEqual_StrStr` (`/Game/Blueprints/BPComponents.Tag` _asbpcomponents) "gear")
    (for _array_element (`self.LinkList`)
      (bind _has (`/Game/Blueprints/Link/BPLink.Has` _array_element self _asbpcomponents))
      (if _has
        (`/Game/Blueprints/Link/BPLink.Disconnect` _array_element)))))

(fn `ConnectGear`
  (params (Other :type "/Game/Blueprints/BPComponents Object Reference"))
  (if (`KismetStringLibrary.EqualEqual_StrStr` (`/Game/Blueprints/BPComponents.Tag` Other) "gear")
    (if (`KismetSystemLibrary.IsValid` (`self.BPHand`))
      (bind _returnvalue (`|GenericCreateObject` "/Game/Blueprints/Link/ImplementedLink/BPGearLink.BPGearLink_C" self))
      (`/Game/Blueprints/Link/BPLink.Connect` _returnvalue self Other)
      (return))))

(fn `ConnectGearWhenStarts`
  (params (`Input Object` :type "/Game/Blueprints/Gear/BPGear Object Reference"))
  (bind _returnvalue (`|GenericCreateObject` "/Game/Blueprints/Link/ImplementedLink/BPGearLink.BPGearLink_C" self))
  (`/Game/Blueprints/Link/BPLink.Connect` _returnvalue self `Input Object`)
  (return))

(fn `DisconnectGear`
  (params (Other :type "/Game/Blueprints/BPComponents Object Reference"))
  (if (`KismetStringLibrary.EqualEqual_StrStr` (`/Game/Blueprints/BPComponents.Tag` Other) "gear")
    (for _array_element (`self.LinkList`)
      (bind _has (`/Game/Blueprints/Link/BPLink.Has` _array_element self Other))
      (if _has
        (`/Game/Blueprints/Link/BPLink.Disconnect` _array_element)))))

(fn `UserConstructionScript`
  (`parent.UserConstructionScript`))