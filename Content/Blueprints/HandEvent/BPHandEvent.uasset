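; BPHandEvent is a Blueprint that defines hand interaction events for catching, holding and releasing with motion controllers.
; HandCatch, HandHold and HandRelease are empty stubs, and IsItSameClass always returns false.
; CanMove holds the only logic, allowing movement only while holding a valid hit actor that is not flagged IsStatic.
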(fn `CanMove`
  (params (IsHolding :type Boolean) (HitActor :type "/Game/Blueprints/BPComponents Object Reference"))
  (returns (CanMove :type Boolean))
  (bind _returnvalue (and IsHolding (`KismetSystemLibrary.IsValid` HitActor)))
  (if _returnvalue
    (if (and _returnvalue (`/Game/Blueprints/BPComponents.isStatic` HitActor))
      _
      (else
        (return true))))
  (return false))

(fn `HandCatch`
  (params (OtherActor :type "/Game/Blueprints/BPComponents Object Reference") (Hand :type "/Game/Blueprints/BPHand Object Reference") (HandSide :type String))
  (return))

(fn `HandHold`
  (params (LeftController :type "MotionControllerComponent Object Reference") (RightController :type "MotionControllerComponent Object Reference"))
  (returns (dump :type "MotionControllerComponent Object Reference"))
  (return null))

(fn `HandRelease`)

(fn `IsItSameClass`
  (params (Event :type "/Game/Blueprints/HandEvent/BPHandEvent Object Reference"))
  (returns (return :type Boolean))
  (return false))