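; VR hand pawn for grabbing and manipulating BPComponents actors with two motion controllers.
; Right trigger and hand overlaps create swappable TouchType event objects to handle catch, hold and release, while Tick repositions held non-static components.
; Controller line traces let thumbsticks rotate components and face buttons toggle motors; grips move the pawn along camera forward or backward.
; Grab logic is mid-rework: older trace-based catch/release functions remain but are unwired.
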(event `self.ReceiveBeginPlay`
  (`HeadMountedDisplayFunctionLibrary.SetTrackingOrigin` "Floor")
  (set `self.HandSideLeft` "LEFT")
  (set `self.HandSideRight` "RIGHT"))

(event `self.ReceiveTick`
  (params (DeltaSeconds :type "Float (single-precision)"))
  (`self.HoldingObjectLeft`)
  (`self.HoldingObjectRight`)
  (`self.HandHold`)
  (`|ExecutionSequence`
    (:`then_0`
      (if (`KismetSystemLibrary.IsValid` (`self.TouchType`))
        (`/Game/Blueprints/HandEvent/BPHandEvent.HandHold` (`self.TouchType`) (`self.MotionController_L`) (`self.MotionController_R`))))
    (:`then_1`
      (`self.MoveHand` DeltaSeconds))))

(event `Key|MotionController_Right_Trigger`
  (params (Key :type "Key Structure"))
  ;[1 1 1] this section will be changed
  (:`Pressed`
    (if (not (`KismetSystemLibrary.IsValid` (`self.TouchType`)))
      (bind _returnvalue (`|GenericCreateObject` "/Game/Blueprints/HandEvent/ImplementedHandEvent/BPTriggerEvent.BPTriggerEvent_C" self))
      (bind _output_get (set `self.TouchType` _returnvalue))
      (`/Game/Blueprints/HandEvent/BPHandEvent.HandCatch` _output_get null null (`self.HandSideRight`))))
  (:`Released`
    (`/Game/Blueprints/HandEvent/BPHandEvent.HandRelease` (`self.TouchType`))
    (set `self.TouchType` null)))

(event `Key|MotionController_Left_Trigger`
  (params (Key :type "Key Structure"))
  ;[1 1 1] this section will be changed
)

(event `Key|MotionController_Right_Grip1`
  (params (Key :type "Key Structure"))
  (:`Pressed`
    (set `self.IsGripHoldingRight` true))
  (:`Released`
    (set `self.IsGripHoldingRight` false)))

(event `Key|MotionController_Left_FaceButton2`
  (params (Key :type "Key Structure"))
  (:`Pressed`
    (`self.ToggleMotorState` (`self.MotionController_L`))))

(event `Key|MotionController_Left_Grip1`
  (params (Key :type "Key Structure"))
  (:`Pressed`
    (set `self.IsGripHoldingLeft` true))
  (:`Released`
    (set `self.IsGripHoldingLeft` false)))

(event `Key|MotionController_Right_FaceButton2`
  (params (Key :type "Key Structure"))
  (:`Pressed`
    (`self.ToggleMotorState` (`self.MotionController_R`))))

(event `Key|MotionController_Left_Thumbstick_Left`
  (params (Key :type "Key Structure"))
  (:`Pressed`
    (`self.TargetAxisRotation` (`self.MotionController_L`) (0.0 0.0 1.0) 1.0)))

(event `Key|MotionController_Left_Thumbstick_Up`
  (params (Key :type "Key Structure"))
  (:`Pressed`
    (`self.TargetAxisRotation` (`self.MotionController_L`) (1.0 0.0 0.0) 1.0)))

(event `Key|MotionController_Right_Thumbstick_Up`
  (params (Key :type "Key Structure"))
  (:`Pressed`
    (`self.TargetAxisRotation` (`self.MotionController_R`) (1.0 0.0 0.0) 1.0)))

(event `Key|MotionController_Right_Thumbstick_Left`
  (params (Key :type "Key Structure"))
  (:`Pressed`
    (`self.TargetAxisRotation` (`self.MotionController_R`) (0.0 0.0 1.0) 1.0)))

(event `Key|MotionController_Left_Thumbstick_Down`
  (params (Key :type "Key Structure"))
  (:`Pressed`
    (`self.TargetAxisRotation` (`self.MotionController_L`) (1.0 0.0 0.0) -1.0)))

(event `Key|MotionController_Left_Thumbstick_Right`
  (params (Key :type "Key Structure"))
  (:`Pressed`
    (`self.TargetAxisRotation` (`self.MotionController_L`) (0.0 0.0 1.0) -1.0)))

(event `Key|MotionController_Right_Thumbstick_Down`
  (params (Key :type "Key Structure"))
  (:`Pressed`
    (`self.TargetAxisRotation` (`self.MotionController_R`) (1.0 0.0 0.0) -1.0)))

(event `Key|MotionController_Right_Thumbstick_Right`
  (params (Key :type "Key Structure"))
  (:`Pressed`
    (`self.TargetAxisRotation` (`self.MotionController_R`) (0.0 0.0 1.0) -1.0)))

(event `self.Touch_L.OnComponentBeginOverlap`
  (params (OverlappedComponent :type "PrimitiveComponent Object Reference") (OtherActor :type "Actor Object Reference") (OtherComp :type "PrimitiveComponent Object Reference") (OtherBodyIndex :type Integer) (bFromSweep :type Boolean) (SweepResult :type "HitResult Structure (by ref)"))
  (bind _touchtype (`self.TouchType`))
  ;[1 1 1] this section will be changed
  (if (`KismetSystemLibrary.IsValid` (`self.TouchType`))
    (bind _return (`/Game/Blueprints/HandEvent/BPHandEvent.IsItSameClass` _touchtype _touchtype))
    (if _return
      (bind _asbpcomponents (cast `/Game/Blueprints/BPComponents` OtherActor :!label _label))
      (bind _returnvalue (`|GenericCreateObject` "/Game/Blueprints/HandEvent/ImplementedHandEvent/BPTouchEvent.BPTouchEvent_C" self))
      (bind _output_get (set `self.TouchType` _returnvalue))
      (`/Game/Blueprints/HandEvent/BPHandEvent.HandCatch` _output_get _asbpcomponents self (`self.HandSideLeft`)))
    (else
      (goto _label))))

(event `self.Touch_R.OnComponentBeginOverlap`
  (params (OverlappedComponent :type "PrimitiveComponent Object Reference") (OtherActor :type "Actor Object Reference") (OtherComp :type "PrimitiveComponent Object Reference") (OtherBodyIndex :type Integer) (bFromSweep :type Boolean) (SweepResult :type "HitResult Structure (by ref)"))
  (bind _touchtype (`self.TouchType`))
  ;[1 1 1] this section will be changed
  (if (`KismetSystemLibrary.IsValid` (`self.TouchType`))
    (bind _return (`/Game/Blueprints/HandEvent/BPHandEvent.IsItSameClass` _touchtype _touchtype))
    (if _return
      (bind _asbpcomponents (cast `/Game/Blueprints/BPComponents` OtherActor :!label _label_2))
      (bind _returnvalue (`|GenericCreateObject` "/Game/Blueprints/HandEvent/ImplementedHandEvent/BPTouchEvent.BPTouchEvent_C" self))
      (bind _output_get (set `self.TouchType` _returnvalue))
      (`/Game/Blueprints/HandEvent/BPHandEvent.HandCatch` _output_get _asbpcomponents self (`self.HandSideRight`)))
    (else
      (goto _label_2))))

(fn `AddHole`
  (params (Hole :type "/Game/Blueprints/Hole/BPHole Object Reference"))
  (`KismetArrayLibrary.Array_Add` (`self.HoleList`) Hole)
  (return))

(fn `CatchObejctLeft`
  (bind _motioncontroller_l (`self.MotionController_L`))
  (bind _returnvalue (`SceneComponent.K2_GetComponentLocation` _motioncontroller_l))
  (if (not (`self.IsHoldingObjectLeft`))
    (set `self.IsHoldingObjectLeft` true)
    (bind (_outhit _returnvalue_2) (`KismetSystemLibrary.LineTraceSingleForObjects` :`Start` _returnvalue :`End` (+ _returnvalue (* (`SceneComponent.GetForwardVector` _motioncontroller_l) 1000.0)) :`ObjectTypes` (`|MakeArray` "ObjectTypeQuery4" :!type "EObjectTypeQuery Enum") :`DrawDebugType` "ForDuration"))
    (if _returnvalue_2
      (bind _asbpcomponents (cast `/Game/Blueprints/BPComponents` (`.HitActor` (`GameplayStatics.BreakHitResult` _outhit))))
      (bind _output_get (set `self.HitActorLeft` _asbpcomponents))
      (`/Game/Blueprints/BPComponents.SetHand` _output_get self (`self.HandSideLeft`))
      (bind _newparam (`self.DistanceHandToTarget` (`SceneComponent.K2_GetComponentLocation` (`self.MotionController_L`)) (`SceneComponent.K2_GetComponentLocation` (`/Game/Blueprints/BPComponents.StaticMesh` (`self.HitActorLeft`)))))
      (set `self.DistanceVectorLeft` _newparam)
      (return))))

(fn `CatchObjectRight`
  (bind _motioncontroller_r (`self.MotionController_R`))
  (bind _returnvalue (`SceneComponent.K2_GetComponentLocation` _motioncontroller_r))
  (if (not (`self.IsHoldingObjectRight`))
    (set `self.IsHoldingObjectRight` true)
    (bind (_outhit _returnvalue_2) (`KismetSystemLibrary.LineTraceSingleForObjects` :`Start` _returnvalue :`End` (+ _returnvalue (* (`SceneComponent.GetForwardVector` _motioncontroller_r) 1000.0)) :`ObjectTypes` (`|MakeArray` "ObjectTypeQuery4" :!type "EObjectTypeQuery Enum") :`DrawDebugType` "ForDuration"))
    (if _returnvalue_2
      (bind _asbpcomponents (cast `/Game/Blueprints/BPComponents` (`.HitActor` (`GameplayStatics.BreakHitResult` _outhit))))
      (bind _output_get (set `self.HitActorRight` _asbpcomponents))
      (`/Game/Blueprints/BPComponents.SetHand` _output_get self (`self.HandSideRight`))
      (bind _newparam (`self.DistanceHandToTarget` (`SceneComponent.K2_GetComponentLocation` (`self.MotionController_R`)) (`SceneComponent.K2_GetComponentLocation` (`/Game/Blueprints/BPComponents.StaticMesh` (`self.HitActorRight`)))))
      (set `self.DistanceVectorRight` _newparam)
      (return))))

(fn `CheckCanMove`
  (params (HoldedSide :type Boolean) (`Hit Actor` :type "/Game/Blueprints/BPComponents Object Reference"))
  (returns (CanMove :type Boolean))
  (bind _returnvalue (and HoldedSide (`KismetSystemLibrary.IsValid` `Hit Actor`)))
  (if _returnvalue
    (if (and _returnvalue (`/Game/Blueprints/BPComponents.isStatic` `Hit Actor`))
      _
      (else
        (return true))))
  (return false))

(fn `DistanceHandToTarget`
  (params (StartLocation :type "Vector Structure") (EndLocation :type "Vector Structure"))
  (returns (NewParam :type "Vector Structure"))
  (return (- EndLocation StartLocation)))

(fn `HandCatch`
  (params (HandSide :type String) (Other :type "Actor Object Reference"))
  (switch `string` HandSide
    (:`LEFT`
      (if (not (`self.IsHoldingObjectLeft`))
        (set `self.IsHoldingObjectLeft` true)
        (bind _asbpcomponents (cast `/Game/Blueprints/BPComponents` Other))
        (bind _output_get (set `self.HitActorLeft` _asbpcomponents))
        (`/Game/Blueprints/BPComponents.SetHand` _output_get self HandSide)
        (return)))
    (:`RIGHT`
      (if (not (`self.IsHoldingObjectRight`))
        (set `self.IsHoldingObjectRight` true)
        (bind _asbpcomponents_2 (cast `/Game/Blueprints/BPComponents` Other))
        (bind _output_get_2 (set `self.HitActorRight` _asbpcomponents_2))
        (`/Game/Blueprints/BPComponents.SetHand` _output_get_2 self HandSide)
        (return)))))

(fn `HandHold`
  (`|ExecutionSequence`
    (:`then_0`
      (bind _canmove (`self.CheckCanMove` (`self.IsHoldingObjectLeft`) (`self.HitActorLeft`)))
      (if _canmove
        (`SceneComponent.K2_SetWorldLocation` (`/Game/Blueprints/BPComponents.StaticMesh` (`self.HitActorLeft`)) (+ (`SceneComponent.K2_GetComponentLocation` (`self.Touch_L`)) (10.0 0.0 10.0)) false false)))))

(fn `HandRelease`)

(fn `HoldingObjectLeft`
  (bind _hitactorleft (`self.HitActorLeft`))
  (if (`self.IsHoldingObjectLeft`)
    (if (`KismetSystemLibrary.IsValid` (`self.HitActorLeft`))
      (if (not (`/Game/Blueprints/BPComponents.isStatic` _hitactorleft))
        (`SceneComponent.K2_SetWorldLocation` (`/Game/Blueprints/BPComponents.StaticMesh` _hitactorleft) (+ (`SceneComponent.K2_GetComponentLocation` (`self.MotionController_L`)) (`self.DistanceVectorLeft`)) false false)
        (return)))))

(fn `HoldingObjectRight`
  (bind _hitactorright (`self.HitActorRight`))
  (if (`self.IsHoldingObjectRight`)
    (if (`KismetSystemLibrary.IsValid` (`self.HitActorRight`))
      (if (not (`/Game/Blueprints/BPComponents.isStatic` _hitactorright))
        (`SceneComponent.K2_SetWorldLocation` (`/Game/Blueprints/BPComponents.StaticMesh` _hitactorright) (+ (`SceneComponent.K2_GetComponentLocation` (`self.MotionController_R`)) (`self.DistanceVectorRight`)) false false)
        (return)))))

(fn `MoveHand`
  (params (DeltaSeconds :type "Float (double-precision)"))
  (`|ExecutionSequence`
    (:`then_0`
      (if (`self.IsGripHoldingRight`)
        (`self.AddMovementInput` (`SceneComponent.GetForwardVector` (`self.Camera`)) (/ (* DeltaSeconds (`self.ForwardSpeed`)) 2.0))))
    (:`then_1`
      (if (`self.IsGripHoldingLeft`)
        (`self.AddMovementInput` (`SceneComponent.GetForwardVector` (`self.Camera`)) (/ (* DeltaSeconds (* (`self.ForwardSpeed`) -1.0)) 2.0))))
    (:`then_2`
      (return))))

(fn `ReleaseObjectLeft`
  (if (`self.IsHoldingObjectLeft`)
    (set `self.IsHoldingObjectLeft` false)
    (if (`KismetSystemLibrary.IsValid` (`self.HitActorLeft`))
      (for _array_element (`self.HoleList`)
        (`/Game/Blueprints/Hole/BPHole.WhenHandRelease` _array_element (`self.HandSideLeft`)))
      (`/Game/Blueprints/BPComponents.SetHand` (`self.HitActorLeft`) null "")
      (set `self.HitActorLeft` null)
      (return))))

(fn `ReleaseObjectRight`
  (if (`self.IsHoldingObjectRight`)
    (set `self.IsHoldingObjectRight` false)
    (if (`KismetSystemLibrary.IsValid` (`self.HitActorRight`))
      (for _array_element (`self.HoleList`)
        (`/Game/Blueprints/Hole/BPHole.WhenHandRelease` _array_element (`self.HandSideRight`)))
      (`/Game/Blueprints/BPComponents.SetHand` (`self.HitActorRight`) null "")
      (set `self.HitActorRight` null)
      (return))))

(fn `RemoveHole`
  (params (Hole :type "/Game/Blueprints/Hole/BPHole Object Reference"))
  (`KismetArrayLibrary.Array_RemoveItem` (`self.HoleList`) Hole)
  (return))

(fn `TargetAxisRotation`
  (params (Controller :type "MotionControllerComponent Object Reference") (Axis :type "Vector Structure") (RotationSign :type "Float (double-precision)"))
  (bind _returnvalue (`SceneComponent.K2_GetComponentLocation` Controller))
  (bind (_outhit _returnvalue_2) (`KismetSystemLibrary.LineTraceSingleForObjects` :`Start` _returnvalue :`End` (+ _returnvalue (* (`SceneComponent.GetForwardVector` Controller) 1000.0)) :`ObjectTypes` (`|MakeArray` "ObjectTypeQuery4" :!type "EObjectTypeQuery Enum") :`DrawDebugType` "ForDuration"))
  (if _returnvalue_2
    (bind _asbpcomponents (cast `/Game/Blueprints/BPComponents` (`.HitActor` (`GameplayStatics.BreakHitResult` _outhit)))
      (:`then`
        (`SceneComponent.K2_AddWorldRotation` (`/Game/Blueprints/BPComponents.StaticMesh` _asbpcomponents) (`KismetMathLibrary.RotatorFromAxisAndAngle` Axis (* (`self.RotationTick`) RotationSign)) false false))
      (:`CastFailed`
        _))
    (return)))

(fn `ToggleMotorState`
  (params (Controller :type "MotionControllerComponent Object Reference"))
  (bind _returnvalue (`SceneComponent.K2_GetComponentLocation` Controller))
  (bind (_outhit _returnvalue_2) (`KismetSystemLibrary.LineTraceSingleForObjects` :`Start` _returnvalue :`End` (+ _returnvalue (* (`SceneComponent.GetForwardVector` Controller) 1000.0)) :`ObjectTypes` (`|MakeArray` "ObjectTypeQuery4" :!type "EObjectTypeQuery Enum") :`DrawDebugType` "ForDuration"))
  (if _returnvalue_2
    (bind _asbpmotor (cast `/Game/Blueprints/BPMotor` (`.HitActor` (`GameplayStatics.BreakHitResult` _outhit)))
      (:`then`
        (`/Game/Blueprints/BPMotor.ToggleEnable` _asbpmotor))
      (:`CastFailed`
        _))
    (return)))

(fn `UserConstructionScript`)